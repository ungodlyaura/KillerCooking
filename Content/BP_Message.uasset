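; BP_Message holds and manages the dialogue for the king's kill orders and the trait-themed customers ordering food from the chef.
; Setup spawns further BP_Message actors as data records, wrapping king orders in a shared intro and outro.
; GetKillTarget picks a random order and splits customer lines into kill and normal pools by matching traits.
; NextCustomer draws a random line from either pool according to ValidVictim.
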(event `Setup`
  (bind _array (`|MakeArray` "Indecisive"))
  (bind _array_2 (`|MakeArray` "Jester"))
  (bind _array_3 (`|MakeArray` "Threat"))
  (bind _array_4 (`|MakeArray` "Rich"))
  (bind _array_5 (`|MakeArray` "Sports"))
  (bind _array_6 (`|MakeArray` "Country"))
  (bind _array_7 (`|MakeArray` "Satanic"))
  (bind _array_8 (`|MakeArray` "Angry"))
  (bind _array_9 (`|MakeArray` "Sad"))
  (bind _array_10 (`|MakeArray` "Worker"))
  ;[1 0.1022 0.07239] Add in new king dialogue/customer dialogue here
  (`self.CreateMessage` "Chef, the wealthy have been flaunting their riches again, while others suffer. Their arrogance is infuriating. Remove anyone who talks or dresses like they're above us. Let them feel what true power is." (`|MakeArray` "Rich") true)
  (`self.CreateMessage` "Those sports fanatics are becoming a nuisance, always shouting and boasting. They distract from my important affairs. If they bring their passion here, end their games for good." (`|MakeArray` "Sports") true)
  (`self.CreateMessage` "Country folk are making demands about land and air quality. If anyone speaks with that country twang, silence them before they stir up more trouble." (`|MakeArray` "Country") true)
  (`self.CreateMessage` "Country folk are making demands about land and air quality. If anyone speaks with that country twang, silence them before they stir up more trouble." (`|MakeArray` "Country") true)
  (`self.CreateMessage` "I’ve heard whispers of those worshipping dark forces. I won’t tolerate their wickedness. Deal with anyone wearing pentagrams or spouting their vile beliefs." (`|MakeArray` "Satanic") true)
  (`self.CreateMessage` "These jesters think they’re funny, mocking me and my kingdom. Their antics are wearing thin. Anyone dressed as a fool or acting like one should be silenced permanently." (`|MakeArray` "Jester") true)
  (`self.CreateMessage` "I’ve been hearing far too many threats against me lately. If anyone speaks of rebellion or harm to my reign, make sure their words are their last." (`|MakeArray` "Threat") true)
  (`self.CreateMessage` "Indecision is weakness, and I won’t stand for it. If anyone hesitates or can’t make up their mind quickly, make the choice for them — permanently." (`|MakeArray` "Indescisive") true)
  (`self.CreateMessage` "People's temperaments are out of control, screaming and causing disruptions. If anyone dares to raise their voice in anger, ensure they never yell again." (`|MakeArray` "Angry") true)
  (`self.CreateMessage` "The kingdom is drowning in tears and complaints. I can’t bear their sorrow any longer. Wipe out anyone who wallows in sadness. They’re dragging us all down." (`|MakeArray` "Sad") true)
  (`self.CreateMessage` "These workers are complaining about their conditions again. Ungrateful, all of them! If anyone speaks of strikes or revolt, eliminate them before they spread their discontent." (`|MakeArray` "Worker") true)
  ;[1 1 1] Comment
  (`self.CreateMessage` "Honestly, I only dine at the finest establishments. Hope this place can meet my high standards. Now, let me have the..." _array_4)
  (`self.CreateMessage` "I’ve just returned from my villa on the coast. Let’s see if your cooking can match what I’m used to. I’ll take the..." _array_4)
  (`self.CreateMessage` "I only eat the best, you know. I expect nothing less than perfection here. Now, bring me the..." _array_4)
  ;[1 1 1] Comment
  (`self.CreateMessage` "Just came from the Serpents' game—what a win! I’m still buzzing with excitement. Gotta celebrate with the..." _array_5)
  (`self.CreateMessage` "Did you see the Serpents’ last match? Medusa’s head shines again! Let me get the..." _array_5)
  (`self.CreateMessage` "The Serpents’ green is everywhere these days, and I’m here to rep the best team! I’ll take the..." _array_5)
  ;[1 1 1] Comment
  (`self.CreateMessage` "Yeehaw! Been working the fields all day, reckon I’ve earned myself a hearty meal. I’ll take the..." _array_6)
  (`self.CreateMessage` "Well, shucks, after a day like today, I’m hungrier than a hog in a cornfield. Get me the..." _array_6)
  (`self.CreateMessage` "Howdy partner, ain't nothin' like a home-cooked meal, but I reckon I’ll settle for the..." _array_6)
  ;[1 1 1] Comment
  (`self.CreateMessage` "The stars aligned last night, a powerful omen. I feel... ravenous today. Give me the..." _array_7)
  (`self.CreateMessage` "The darkness calls, and I must feast to regain my strength. Prepare for me the..." _array_7)
  (`self.CreateMessage` "I've spoken to the dark forces, and they’ve guided me here. Now, I need the..." _array_7)
  ;[1 1 1] Comment
  (`self.CreateMessage` "Oh ho ho! You should’ve seen the trick I pulled today—had everyone in stitches. Now, serve me the..." _array_2)
  (`self.CreateMessage` "Oh, the laughs I had today! But I need food for my next balancing act. I’ll take the..." _array_2)
  (`self.CreateMessage` "Juggling’s hard work, you know! Time for a little treat—fetch me the..." _array_2)
  ;[1 1 1] Comment
  (`self.CreateMessage` "I’ve heard some whispers about the king... He’s not as untouchable as he thinks. Before I go deal with him, I’ll have the..." _array_3)
  (`self.CreateMessage` "The king’s days are numbered. But first, I need to fuel up. I’ll take the..." _array_3)
  (`self.CreateMessage` "It’s about time someone took out that \"almighty\" rat... I’ll need my strength. Give me the..." _array_3)
  ;[1 1 1] Comment
  (`self.CreateMessage` "Unbelievable! This day can’t get any worse. Just hurry up and give me the..." _array_8)
  (`self.CreateMessage` "This is ridiculous! I don’t have time for your nonsense—just give me the..." _array_8)
  (`self.CreateMessage` "I’ve had enough! This day is the worst, and I don’t have patience left. Bring me the..." _array_8)
  ;[1 1 1] Comment
  (`self.CreateMessage` "Nothing’s been going right lately... I just need something comforting to eat. Can I have the..." _array_9)
  (`self.CreateMessage` "Everything’s been so hard lately... I just want something warm to eat. I’ll have the..." _array_9)
  (`self.CreateMessage` "I don’t even know why I’m here. Just... bring me my last and final meal, the..." _array_9)
  ;[1 1 1] Comment
  (`self.CreateMessage` "Uhhh... I can’t decide... Maybe the... No, wait! What was I thinking? I’ll have the..." _array)
  (`self.CreateMessage` "Hmm... maybe this, or that? Oh, I don’t know! What’s easiest? I’ll have the..." _array)
  (`self.CreateMessage` "Wait, I was sure I wanted something, but now I’m not so sure. Maybe I’ll go with the..." _array)
  ;[1 1 1] Comment
  (`self.CreateMessage` "I’ve been on my feet all day, can’t waste time or i'll get fired. Just grab me the..." _array_10)
  (`self.CreateMessage` "I’ve been working double shifts—barely had time to breathe. Just get me the..." _array_10)
  (`self.CreateMessage` "I can’t waste any time here, my shift’s almost over. I’ll take the..." _array_10)
  (`self.GetKillTarget`))

(event `GetKillTarget`
  (bind _killreasons (`self.KillReasons`))
  ;[1 1 1] Get king dialogue and sort messages
  (if (`KismetSystemLibrary.IsValid` (`|GetArrayItem` (`self.KillReasons`)))
    (set `self.KillTarget` (`|GetArrayItem` _killreasons (`KismetMathLibrary.RandomIntegerInRange` 0 (- (`KismetArrayLibrary.Array_Length` _killreasons) 1))))
    (for _array_element (`self.Messages`)
      (set `self.bTempFound` false)
      (for _array_element_2 (`/Game/BP_Message.Trait` _array_element)
        (if (`KismetArrayLibrary.Array_Contains` (`/Game/BP_Message.Trait` (`self.KillTarget`)) _array_element_2)
          (set `self.bTempFound` true)))
      (if (`self.bTempFound`)
        (`KismetArrayLibrary.Array_Add` (`self.KillMessages`) _array_element)
        (set `/Game/BP_Message.bKillTarget` true _array_element)
        (else
          (`KismetArrayLibrary.Array_Add` (`self.NormalMessages`) _array_element))))
    (else
      (`KismetSystemLibrary.PrintString` "Forget to add messages?"))))

(event `CreateMessage`
  (params (Message :type String) (Traits :type "Array of String") (bKillMessage :type Boolean))
  ;[1 1 1] create message object
  (bind _returnvalue (`|SpawnActorFromClass` "BP_Message_C" (`KismetMathLibrary.Conv_VectorToTransform` (0.0 0.0 0.0)) "Undefined" "MultiplyWithRoot" null null))
  (set `/Game/BP_Message.Message` Message _returnvalue)
  (set `/Game/BP_Message.Trait` Traits _returnvalue)
  (if bKillMessage
    (set `/Game/BP_Message.Message` (`KismetStringLibrary.Concat_StrStr` (`KismetStringLibrary.Concat_StrStr` "Dearest chef, \nI have another task for you. The kingdom is full of nuisances lately, and I trust you to handle them swiftly. \n \n" Message) " \n \nDo this, and our land will be much more peaceful. I expect nothing less than perfection from you.") _returnvalue)
    (`KismetArrayLibrary.Array_Add` (`self.KillReasons`) _returnvalue)
    (else
      (`KismetArrayLibrary.Array_Add` (`self.Messages`) _returnvalue))))

(event `NextCustomer`
  (params (bValidVictim :type Boolean))
  (bind _normalmessages (`self.NormalMessages`))
  (bind _killmessages (`self.KillMessages`))
  (bind _currentcustomer (`self.CurrentCustomer`))
  ;[1 1 1] Get Next Customer
  (if (`KismetSystemLibrary.IsValid` _currentcustomer)
    (`KismetArrayLibrary.Array_RemoveItem` (`self.Messages`) _currentcustomer))
  (if bValidVictim
    (set `self.CurrentCustomer` (`|GetArrayItem` _killmessages (`KismetMathLibrary.RandomInteger` (`KismetArrayLibrary.Array_Length` _killmessages))))
    (set `self.bKillTarget` true)
    (else
      (set `self.CurrentCustomer` (`|GetArrayItem` _normalmessages (`KismetMathLibrary.RandomInteger` (`KismetArrayLibrary.Array_Length` _normalmessages)))))))

(fn `UserConstructionScript`)