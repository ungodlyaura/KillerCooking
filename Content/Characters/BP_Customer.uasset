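; BP_Customer is a customer character that shows a different look depending on its assigned trait.
; A Setup event switches on the Trait (Sports, Country, Rich, Jester, Threat or Satanic) and unhides the matching component along with its children.
; It only reveals the chosen variant and does not hide the others, and BeginPlay, overlap, Tick and the construction script are empty.
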(event `Setup`
  (params (Trait :type String))
  (switch `string` Trait
    (:`Sports`
      (`SceneComponent.SetHiddenInGame` (`self.Sports`) false true))
    (:`Country`
      (`SceneComponent.SetHiddenInGame` (`self.Country`) false true))
    (:`Rich`
      (`SceneComponent.SetHiddenInGame` (`self.Rich`) false true))
    (:`Jester`
      (`SceneComponent.SetHiddenInGame` (`self.Jester`) false true))
    (:`Threat`
      (`SceneComponent.SetHiddenInGame` (`self.Threat`) false true))
    (:`Satanic`
      (`SceneComponent.SetHiddenInGame` (`self.Satanic`) false true))))

(fn `UserConstructionScript`)