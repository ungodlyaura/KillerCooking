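; BP_GhostCharacter is an AI ghost that costs the player one health on spawn and roams between floor MoveSpots.
; It claims a random unoccupied spot, walks there with AIMoveTo, then waits on the player's seconds counter before choosing another.
; StartAttack has a coin-flip chance to flag a Giver block at its current spot as PoisonNext; branches for other block types are empty.
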(event `StartAttack`
  (bind _currentspot (`self.CurrentSpot`))
  (bind _block (`/Game/Blocks/MoveSpot.Block` _currentspot))
  (bind _type (`/Game/Blocks/AInteractable.Type` _block))
  (if (== (`KismetMathLibrary.RandomInteger` 2) 0)
    (if (`KismetSystemLibrary.IsValid` _currentspot)
      (if (`KismetStringLibrary.EqualEqual_StrStr` _type "Giver")
        (set `/Game/Blocks/AInteractable.PoisonNext` true _block)
        (elif (`KismetStringLibrary.EqualEqual_StrStr` _type "Cooker")
          _
          (elif (`KismetStringLibrary.EqualEqual_StrStr` _type "Holder")
            _
            (elif (`KismetSystemLibrary.IsValid` (`/Game/Blocks/AInteractable.Holding` _block))
              _))))
      (elif true
        _))))

(event `GoNewSpot`
  (bind _currentspot (`self.CurrentSpot`))
  (bind (_returnvalue_x _returnvalue_y _returnvalue_z) (`KismetMathLibrary.BreakVector` (`self.K2_GetActorLocation` self)))
  (if (`KismetSystemLibrary.IsValid` _currentspot)
    (set `/Game/Blocks/MoveSpot.Ghost` null _currentspot))
  (set `self.CurrentSpot` null)
  (while (== (`KismetSystemLibrary.IsValid` (`self.CurrentSpot`)) false)
    (bind _output_get (set `self.CurrentSpot` (`KismetArrayLibrary.Array_Random` (`self.FloorSpots`))))
    (if (`KismetSystemLibrary.IsValid` (`/Game/Blocks/MoveSpot.Ghost` _output_get))
      (set `self.CurrentSpot` null)
      (else
        (set `/Game/Blocks/MoveSpot.Ghost` self _output_get))))
  (bind (_returnvalue_x_2 _returnvalue_y_2) (`KismetMathLibrary.BreakVector` (`self.K2_GetActorLocation` _output_get)))
  (bind _movementresult (`|AIMoveTo` self (`KismetMathLibrary.MakeVector` _returnvalue_x_2 _returnvalue_y_2 _returnvalue_z) _output_get 50.0 true)
    (:`OnSuccess`
      _)
    (:`OnFail`
      (`KismetSystemLibrary.PrintString` (`|GetEnumeratorNameAsString` _movementresult))))
  (set `self.CapturedTime` (`/Game/Characters/BP_PlayerCharacter.Seconds` (`self.Player`))))

(event `self.ReceiveBeginPlay`
  (bind _asbp_player_character (cast `/Game/Characters/BP_PlayerCharacter` (`GameplayStatics.GetPlayerCharacter` 0)))
  (bind _output_get (set `self.Player` _asbp_player_character))
  (set `/Game/Characters/BP_PlayerCharacter.Health` (- (`/Game/Characters/BP_PlayerCharacter.Health` _output_get) 1) _output_get)
  (`/Game/UI/W_GameUI.RefreshHealth` (`/Game/Characters/BP_PlayerCharacter.GameUI` _output_get))
  (bind _outactors (`GameplayStatics.GetAllActorsOfClass` "/Game/Blocks/MoveSpot.MoveSpot_C"))
  (set `self.FloorSpots` _outactors)
  (`self.GoNewSpot`))

(event `self.ReceiveTick`
  (params (DeltaSeconds :type "Float (single-precision)"))
  (bind _capturedtime (`self.CapturedTime`))
  (if (> _capturedtime -1.0)
    (if (> (`/Game/Characters/BP_PlayerCharacter.Seconds` (`self.Player`)) (+ _capturedtime (`self.WaitTime`)))
      (set `self.CapturedTime` -1.0)
      (`self.GoNewSpot`))))

(fn `UserConstructionScript`)