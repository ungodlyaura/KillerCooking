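; BP_Goblin is a goblin character Blueprint with a visual component for each trait: Sports, Country, Rich, Jester, Threat and Satanic.
; Its Setup event takes a Trait and switches on it to hide the matching component and that component's children.
; It only ever hides components, and the construction script and other events are empty.
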(event `Setup`
  (params (Trait :type String))
  (switch `string` Trait
    (:`Sports`
      (`SceneComponent.SetVisibility` (`self.Sports`) false true))
    (:`Country`
      (`SceneComponent.SetVisibility` (`self.Country`) false true))
    (:`Rich`
      (`SceneComponent.SetVisibility` (`self.Rich`) false true))
    (:`Jester`
      (`SceneComponent.SetVisibility` (`self.Jester`) false true))
    (:`Threat`
      (`SceneComponent.SetVisibility` (`self.Threat`) false true))
    (:`Satanic`
      (`SceneComponent.SetVisibility` (`self.Satanic`) false true))))

(fn `UserConstructionScript`)