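; BP_Bomb is a timed bomb actor that damages the player if they are in range when it goes off.
; Overlap begin and end events track whether the player character is touching it.
; Four seconds after BeginPlay it calls TakeDamage on player 0's character if touching, then destroys itself.
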(event `self.ReceiveBeginPlay`
  (`KismetSystemLibrary.Delay` 4.0)
  (if (`self.bPlayerTouching`)
    (bind _asbp_player_character (cast `/Game/Characters/BP_PlayerCharacter` (`GameplayStatics.GetPlayerCharacter` 0)))
    (`/Game/Characters/BP_PlayerCharacter.TakeDamage` _asbp_player_character))
  (`self.K2_DestroyActor`))

(event `self.ReceiveActorBeginOverlap`
  (params (OtherActor :type "Actor Object Reference"))
  (cast `/Game/Characters/BP_PlayerCharacter` OtherActor)
  (set `self.bPlayerTouching` true))

(event `self.ReceiveActorEndOverlap`
  (params (OtherActor :type "Actor Object Reference"))
  (cast `/Game/Characters/BP_PlayerCharacter` OtherActor)
  (set `self.bPlayerTouching` false))

(fn `UserConstructionScript`)