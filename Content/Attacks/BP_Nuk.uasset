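; BP_Nuk is a timed bomb attack that removes one point of player health and destroys itself when its countdown expires, unless disarmed.
; Tick counts down the fuse and shows the seconds left with a hold-E prompt in a dynamic text widget.
; Holding interact locks player movement, turns them toward the bomb and builds disarm progress until the actor is destroyed.
; Releasing early restores movement and resets progress.
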(event `self.GameStart`
  (bind _asw_progress_bar (cast `/Game/UI/W_ProgressBar` (`WidgetComponent.GetWidget` (`self.HoldProgress`))))
  (set `/Game/UI/W_ProgressBar.InteractableOwner` self _asw_progress_bar))

(event `self.ReceiveTick`
  (params (DeltaSeconds :type "Float (single-precision)"))
  (bind _player (`self.Player`))
  (bind _explodetime (`self.ExplodeTime`))
  (if (<= _explodetime 0.0)
    (set `/Game/Characters/BP_PlayerCharacter.Health` (- (`/Game/Characters/BP_PlayerCharacter.Health` _player) 1) _player)
    (`/Game/UI/W_GameUI.RefreshHealth` (`/Game/Characters/BP_PlayerCharacter.GameUI` _player))
    (`self.K2_DestroyActor`)
    (else
      (bind _asw_dynamic_text (cast `/Game/UI/W_DynamicText` (`WidgetComponent.GetUserWidgetObject` (`self.DynamicText`))))
      (`/Game/UI/W_DynamicText.ChangeText` _asw_dynamic_text (`KismetTextLibrary.Conv_StringToText` (`KismetStringLibrary.Concat_StrStr` "Hold 'E' To Disarm! \n" (`KismetTextLibrary.Conv_TextToString` (`KismetTextLibrary.Conv_IntToText` (`KismetMathLibrary.FFloor` _explodetime))))))
      (set `self.ExplodeTime` (- (`self.ExplodeTime`) DeltaSeconds))
      (if (`self.bProgressBarShown`)
        (bind _output_get (set `self.ActionProgress` (+ (`self.ActionProgress`) DeltaSeconds)))
        (if (>= _output_get (`self.ActionFinishTime`))
          (set `/Game/Characters/BP_PlayerCharacter.bCanMove` true (`self.Player`))
          (`self.K2_DestroyActor`))))))

(event `self.OnInteract`
  (bind _player (`self.Player`))
  (set `/Game/Characters/BP_PlayerCharacter.bCanMove` false _player)
  (set `self.bProgressBarShown` true)
  (`self.K2_SetActorRotation` _player (`KismetMathLibrary.Conv_VectorToRotator` (`KismetMathLibrary.GreaterGreater_VectorRotator` (`KismetMathLibrary.Normal` (* (- (`self.K2_GetActorLocation` self) (`self.K2_GetActorLocation` _player)) (1.0 1.0 0.0))))) false))

(event `self.OnReleaseInteract`
  (if (`self.bProgressBarShown`)
    (set `self.bProgressBarShown` false)
    (set `/Game/Characters/BP_PlayerCharacter.bCanMove` true (`self.Player`))
    (set `self.ActionProgress` 0.0)))

(fn `UserConstructionScript`
  (`parent.UserConstructionScript`))