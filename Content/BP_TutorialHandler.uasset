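; Tutorial sequencer for the cooking game, showing contextual popup hints as the player learns to serve customers, prep, cook and submit dishes.
; Creates a W_TutorialPopups widget, then gameplay events toggle its hint visibility, most gated by a TutorialStep counter that enforces order.
; A separate poison hint appears after cooking stops if the first dish order is a poison target and PoisonDone is false.
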(event `self.ReceiveBeginPlay`
  (bind _returnvalue (`|CreateWidget` "/Game/UI/W_TutorialPopups.W_TutorialPopups_C"))
  (bind _output_get (set `self.PopupUI` _returnvalue))
  (`UserWidget.AddToViewport` _output_get 0)
  (bind _asbp_third_person_character (cast `/Game/ThirdPerson/Blueprints/BP_ThirdPersonCharacter` (`GameplayStatics.GetPlayerCharacter` 0)))
  (set `self.Player` _asbp_third_person_character)
  (set `Widget.Visibility` "Visible" (`/Game/UI/W_TutorialPopups.Message` (`self.PopupUI`))))

(event `KingMessageClosed`
  (bind _popupui (`self.PopupUI`))
  (if (== (`self.TutorialStep`) 0)
    (`Widget.RemoveFromParent` (`self.PopupUI`))
    (bind _returnvalue (`|CreateWidget` "/Game/UI/W_TutorialPopups.W_TutorialPopups_C"))
    (bind _output_get (set `self.PopupUI` _returnvalue))
    (`UserWidget.AddToViewport` _output_get 0)
    (set `Widget.Visibility` "Hidden" (`/Game/UI/W_TutorialPopups.Message` _popupui))
    (set `Widget.Visibility` "Visible" (`/Game/UI/W_TutorialPopups.Move` _popupui))
    (set `Widget.Visibility` "Visible" (`/Game/UI/W_TutorialPopups.Customer` _popupui))
    (set `self.TutorialStep` (+ (`self.TutorialStep`) 1))))

(event `PlayerMoved`
  (set `Widget.Visibility` "Hidden" (`/Game/UI/W_TutorialPopups.Move` (`self.PopupUI`))))

(event `CustomerTalk`
  (bind _popupui (`self.PopupUI`))
  (if (== (`self.TutorialStep`) 1)
    (set `Widget.Visibility` "Hidden" (`/Game/UI/W_TutorialPopups.Customer` _popupui))
    (set `Widget.Visibility` "Visible" (`/Game/UI/W_TutorialPopups.Pickup` _popupui))
    (set `self.TutorialStep` (+ (`self.TutorialStep`) 1))))

(event `IngredientPickup`
  (bind _popupui (`self.PopupUI`))
  (if (== (`self.TutorialStep`) 2)
    (set `Widget.Visibility` "Hidden" (`/Game/UI/W_TutorialPopups.Pickup` _popupui))
    (set `Widget.Visibility` "Visible" (`/Game/UI/W_TutorialPopups.Chop` _popupui))
    (set `self.TutorialStep` (+ (`self.TutorialStep`) 1))))

(event `IngredientChopped`
  (bind _popupui (`self.PopupUI`))
  (if (== (`self.TutorialStep`) 3)
    (set `Widget.Visibility` "Hidden" (`/Game/UI/W_TutorialPopups.Chop` _popupui))
    (set `Widget.Visibility` "Visible" (`/Game/UI/W_TutorialPopups.Water` _popupui))
    (set `Widget.Visibility` "Visible" (`/Game/UI/W_TutorialPopups.Stick` _popupui))
    (set `Widget.Visibility` "Visible" (`/Game/UI/W_TutorialPopups.Combine` _popupui))
    (set `Widget.Visibility` "Visible" (`/Game/UI/W_TutorialPopups.Grill` _popupui))
    (set `Widget.Visibility` "Visible" (`/Game/UI/W_TutorialPopups.Stove` _popupui))
    (set `Widget.Visibility` "Visible" (`/Game/UI/W_TutorialPopups.Oven` _popupui))
    (set `self.TutorialStep` (+ (`self.TutorialStep`) 1))))

(event `StartedCooking`
  (bind _popupui (`self.PopupUI`))
  (if (== (`self.TutorialStep`) 4)
    (set `Widget.Visibility` "Hidden" (`/Game/UI/W_TutorialPopups.Water` _popupui))
    (set `Widget.Visibility` "Hidden" (`/Game/UI/W_TutorialPopups.Stick` _popupui))
    (set `Widget.Visibility` "Hidden" (`/Game/UI/W_TutorialPopups.Combine` _popupui))
    (set `Widget.Visibility` "Hidden" (`/Game/UI/W_TutorialPopups.Grill` _popupui))
    (set `Widget.Visibility` "Hidden" (`/Game/UI/W_TutorialPopups.Stove` _popupui))
    (set `Widget.Visibility` "Hidden" (`/Game/UI/W_TutorialPopups.Oven` _popupui))
    (set `Widget.Visibility` "Visible" (`/Game/UI/W_TutorialPopups.Score` _popupui))
    (set `self.TutorialStep` (+ (`self.TutorialStep`) 1))))

(event `FoodCombined`)

(event `StoppedCooking`
  (bind _popupui (`self.PopupUI`))
  (if (`self.PoisonDone`)
    _
    (elif (`/Game/Food/ACustomer.PoisonTarget` (`|GetArrayItem` (`/Game/ThirdPerson/Blueprints/BP_ThirdPersonCharacter.DishOrders` (`self.Player`))))
      (set `Widget.Visibility` "Visible" (`/Game/UI/W_TutorialPopups.Poison` (`self.PopupUI`)))))
  (if (== (`self.TutorialStep`) 5)
    (set `Widget.Visibility` "Visible" (`/Game/UI/W_TutorialPopups.Trash` _popupui))
    (set `Widget.Visibility` "Visible" (`/Game/UI/W_TutorialPopups.Submit` _popupui))
    (set `Widget.Visibility` "Hidden" (`/Game/UI/W_TutorialPopups.Score` _popupui))
    (set `self.TutorialStep` (+ (`self.TutorialStep`) 1))))

(event `DishPoisoned`
  (set `Widget.Visibility` "Hidden" (`/Game/UI/W_TutorialPopups.Poison` (`self.PopupUI`))))

(event `FoodSubmitted`
  (bind _popupui (`self.PopupUI`))
  (if (== (`self.TutorialStep`) 6)
    (set `Widget.Visibility` "Hidden" (`/Game/UI/W_TutorialPopups.Trash` _popupui))
    (set `Widget.Visibility` "Hidden" (`/Game/UI/W_TutorialPopups.Submit` _popupui))
    (set `Widget.Visibility` "Hidden" (`/Game/UI/W_TutorialPopups.Poison` (`self.PopupUI`)))
    (set `self.TutorialStep` (+ (`self.TutorialStep`) 1))))

(fn `UserConstructionScript`)