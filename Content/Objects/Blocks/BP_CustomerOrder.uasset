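; BP_CustomerOrder is an interactable block where the player collects dish orders from waiting customers.
; A Tick frame counter flags a waiting customer and swaps the Cube material once it passes GoalTick.
; EEvent toggles player movement and moves the first CameraActor between two fixed views.
; On entering, a waiting customer adds a random FinishedDishes entry to the character's DishOrders and restarts the counter with a random goal.
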(event `self.ReceiveTick`
  (params (DeltaSeconds :type "Float (single-precision)"))
  (bind _currenttick (`self.CurrentTick`))
  (if (not (`self.CustomerWaiting`))
    (set `self.CurrentTick` (+ _currenttick 1))
    (if (> _currenttick (`self.GoalTick`))
      (set `self.CustomerWaiting` true)
      (`PrimitiveComponent.SetMaterial` (`self.Cube`) 0 "/Engine/MapTemplates/Materials/BasicAsset03.BasicAsset03"))))

(event `self.E_Event`
  (bind _finisheddishes (`self.FinishedDishes`))
  (bind _returnvalue (- (`KismetArrayLibrary.Array_Length` _finisheddishes) 1))
  (bind _asbp_third_person_character (cast `/Game/ThirdPerson/Blueprints/BP_ThirdPersonCharacter` (`GameplayStatics.GetPlayerCharacter` 0)))
  (bind _outactors (`GameplayStatics.GetAllActorsOfClass` "/Script/Engine.CameraActor"))
  (if (`/Game/ThirdPerson/Blueprints/BP_ThirdPersonCharacter.CanMove` _asbp_third_person_character)
    (set `/Game/ThirdPerson/Blueprints/BP_ThirdPersonCharacter.CanMove` false _asbp_third_person_character)
    (`self.K2_SetActorLocationAndRotation` (`|GetArrayItem` _outactors) (950.0 1380.0 150.0) (struct :`Yaw` 90.0) false false)
    (if (`self.CustomerWaiting`)
      (set `self.CustomerWaiting` false)
      (`PrimitiveComponent.SetMaterial` (`self.Cube`) 0 "/Engine/MapTemplates/Materials/BasicAsset01.BasicAsset01")
      (set `self.CurrentTick` 0)
      (set `self.GoalTick` (`KismetMathLibrary.FTrunc` (* (`KismetMathLibrary.Conv_Int64ToDouble` (`KismetMathLibrary.RandomInteger64InRange` 10 15)) 100.0)))
      (bind _dishorders (`/Game/ThirdPerson/Blueprints/BP_ThirdPersonCharacter.DishOrders` _asbp_third_person_character))
      (`KismetArrayLibrary.Array_Insert` _dishorders (`|GetArrayItem` _finisheddishes (`KismetMathLibrary.RandomIntegerInRange` 0 _returnvalue)) _returnvalue)
      (`KismetSystemLibrary.PrintString` (`|GetArrayItem` _dishorders)))
    (else
      (set `/Game/ThirdPerson/Blueprints/BP_ThirdPersonCharacter.CanMove` true _asbp_third_person_character)
      (`self.K2_SetActorLocationAndRotation` (`|GetArrayItem` _outactors) (400.0 1110.0 510.0) (struct :`Pitch` 310.0) false false))))

(fn `UserConstructionScript`
  (`parent.UserConstructionScript`))