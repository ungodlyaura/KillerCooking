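; BP_Stove is a block that cooks the item it holds and eventually burns it into charcoal.
; Each tick it adds one to the held item's Heat, so heating speed depends on frame rate.
; Past a fixed threshold it destroys the item, spawns BP_Charcoal just above itself and holds that instead.
; Pickup updates the block and player holding state through SetBlockHolding and SetPlayerHolding.
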(event `self.ReceiveTick`
  (params (DeltaSeconds :type "Float (single-precision)"))
  (bind _holding (`self.Holding`))
  (if (`KismetSystemLibrary.IsValid` _holding)
    (bind _output_get (set `/Game/Food.Heat` (+ 1 (`/Game/Food.Heat` _holding)) _holding))
    (if (> _output_get 1000)
      (`self.K2_DestroyActor` _holding)
      (bind _returnvalue (`|SpawnActorFromClass` "/Game/Objects/Food/BP_Charcoal.BP_Charcoal_C" (`KismetMathLibrary.Conv_VectorToTransform` (+ (`self.K2_GetActorLocation`) (0.0 0.0 50.0))) "Undefined" "MultiplyWithRoot" null null))
      (set `self.Holding` _returnvalue))))

(event `self.Pickup`
  (`self.SetBlockHolding`)
  (`self.SetPlayerHolding` false))

(fn `UserConstructionScript`
  (`parent.UserConstructionScript`))